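; Player character Blueprint for CCD that maps input to interaction, movement, view toggle, equipment use and switching (Hands, Mop, Scanner), and eye closing.
; BeginPlay adds the default Enhanced Input context and creates emote and item wheel widgets, shown while their input is held.
; Releasing applies the wheel's selection, and playing an emote leaves first-person view.
; Hardcoded keys handle several actions, including a Q toggle between Die and Revive.
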(event Custom|OnDeath
  ;[0.15 0.15 0.15 0.5] 사망 이벤트
  (Utilities|FlowControl|DoOnce false
    (:Completed
      (Development|PrintString "DEAD"))))

(event Input|EnhancedActionEvents|EnhancedInputActionIA_ItemWheel
  (params (ActionValue :type Boolean) (ElapsedSeconds :type Float%20%28double-precision%29) (TriggeredSeconds :type Float%20%28double-precision%29) (InputAction :type Input%20Action%20Object%20Reference :default "/Game/_CCD/Input/IA_ItemWheel.IA_ItemWheel"))
  (:Started
    (CallFunction|OpenItemWheel))
  (:Completed
    (CallFunction|CloseItemWheel)))

(event Input|EnhancedActionEvents|EnhancedInputActionIA_UseEquipment
  (params (ActionValue :type Boolean) (ElapsedSeconds :type Float%20%28double-precision%29) (TriggeredSeconds :type Float%20%28double-precision%29) (InputAction :type Input%20Action%20Object%20Reference :default "/Game/_CCD/Input/IA_UseEquipment.IA_UseEquipment"))
  ;[0.15 0.15 0.15 0.5] Input Actions
  (:Started
    (Class|CCDCharacter|UseEquipment)))

(event Input|EnhancedActionEvents|EnhancedInputActionIA_EmoteWheel
  (params (ActionValue :type Boolean) (ElapsedSeconds :type Float%20%28double-precision%29) (TriggeredSeconds :type Float%20%28double-precision%29) (InputAction :type Input%20Action%20Object%20Reference :default "/Game/_CCD/Input/IA_EmoteWheel.IA_EmoteWheel"))
  (:Started
    (CallFunction|OpenEmote))
  (:Completed
    (CallFunction|CloseEmote)))

(event Input|EnhancedActionEvents|EnhancedInputActionIA_Interact
  (params (ActionValue :type Boolean) (ElapsedSeconds :type Float%20%28double-precision%29) (TriggeredSeconds :type Float%20%28double-precision%29) (InputAction :type Input%20Action%20Object%20Reference :default "/Game/_CCD/Input/IA_Interact.IA_Interact"))
  ;[0.15 0.15 0.15 0.5] Input Actions
  (:Started
    (Class|CCDCharacter|PerformInteract)))

(event EventBeginPlay
  ;[0.15 0.15 0.15 0.5] IMC
  (bind _asplayer_controller (Utilities|Casting|CastToPlayerController (Pawn|GetController)))
  (Input|AddMappingContext (PlayerController|LocalPlayerSubsystems|GetEnhancedInputLocalPlayerSubsystem _asplayer_controller) "/Game/_CCD/Input/IMC_Default.IMC_Default" 1 "(bIgnoreAllPressedKeysUntilRelease=True,bForceImmediately=False,bNotifyUserSettings=False)")
  (bind _returnvalue (UserInterface|CreateWidget "/Game/_CCD/UI/ItemWheel/WBP_EmoteSelect.WBP_EmoteSelect_C" (Game|GetPlayerController 0)))
  (Variables|Default|SetEmote _returnvalue)
  (bind _returnvalue_2 (UserInterface|CreateWidget "/Game/_CCD/UI/ItemWheel/WBP_ItemWheel.WBP_ItemWheel_C" (Game|GetPlayerController 0)))
  (Variables|Default|SetItem%20Wheel _returnvalue_2))

(event Collision|EventActorBeginOverlap
  (params (OtherActor :type Actor%20Object%20Reference)))

(event EventTick
  (params (DeltaSeconds :type Float%20%28single-precision%29)))

(event Input|KeyboardEvents|1
  (params (Key :type Key%20Structure :default "None"))
  ;[0.15 0.15 0.15 0.5] Input Actions
  (:Pressed
    (Class|CCDCharacter|SwitchEquipment "EES_Hands")))

(event Input|KeyboardEvents|4
  (params (Key :type Key%20Structure :default "None"))
  ;[0.15 0.15 0.15 0.5] Input Actions
  (:Pressed
    (Class|CCDCharacter|ToggleView)))

(event Input|KeyboardEvents|2
  (params (Key :type Key%20Structure :default "None"))
  ;[0.15 0.15 0.15 0.5] Input Actions
  (:Pressed
    (Class|CCDCharacter|SwitchEquipment "EES_Mop")))

(event Input|KeyboardEvents|3
  (params (Key :type Key%20Structure :default "None"))
  ;[0.15 0.15 0.15 0.5] Input Actions
  (:Pressed
    (Class|CCDCharacter|SwitchEquipment "EES_Scanner")))

(event Input|KeyboardEvents|LeftShift
  (params (Key :type Key%20Structure :default "None"))
  ;[0.15 0.15 0.15 0.5] Input Actions
  (:Pressed
    (Class|CCDCharacter|SetRunning true))
  (:Released
    (Class|CCDCharacter|SetRunning false)))

(event Input|KeyboardEvents|LeftCtrl
  (params (Key :type Key%20Structure :default "None"))
  ;[0.15 0.15 0.15 0.5] Input Actions
  (:Pressed
    (if (Variables|Default|GetbIsCrouched)
      (Character|UnCrouch)
      (else
        (Character|Crouch)))))

(event Input|KeyboardEvents|Q
  (params (Key :type Key%20Structure :default "None"))
  ;[0.15 0.15 0.15 0.5] 사망 이벤트
  (:Pressed
    (Utilities|FlowControl|FlipFlop
      (:A
        (Class|CCDCharacter|Die))
      (:B
        (Class|CCDCharacter|Revive)))))

(event Input|KeyboardEvents|X
  (params (Key :type Key%20Structure :default "None"))
  ;[0.15 0.15 0.15 0.5] 눈감기 (쿨다운 초기화용)
  (:Pressed
    (Class|CCDCharacter|CloseEye)))

(event Input|KeyboardEvents|SpaceBar
  (params (Key :type Key%20Structure :default "None"))
  ;[0.15 0.15 0.15 0.5] Input Actions
  (:Pressed
    (Character|Jump)))

(fn ConstructionScript)

(fn OpenEmote
  (bind _returnvalue (Game|GetPlayerController 0))
  (if (Utilities|IsValid (Variables|Default|GetEmote))
    _
    (else
      (bind _returnvalue_2 (UserInterface|CreateWidget "/Game/_CCD/UI/ItemWheel/WBP_EmoteSelect.WBP_EmoteSelect_C" (Game|GetPlayerController 0)))
      (Variables|Default|SetEmote _returnvalue_2)))
  (UserInterface|Viewport|AddtoViewport (Variables|Default|GetEmote) 0)
  (Input|SetInputModeGameandUI _returnvalue 0 "LockAlways" true false)
  (Variables|/Script/Engine.PlayerController|SetbShowMouseCursor _returnvalue false))

(fn CloseEmote
  (bind _returnvalue (Game|GetPlayerController 0))
  (bind _emote (Variables|Default|GetEmote))
  (bind (_sectionname _playemote_) (Default|ReturnEmoteResult _emote))
  (Widget|RemovefromParent _emote)
  (Input|SetInputModeGameOnly _returnvalue false)
  (Variables|/Script/Engine.PlayerController|SetbShowMouseCursor _returnvalue false)
  (if _playemote_
    (Class|CCDCharacter|PerformEmote _sectionname)
    (if (Class|CCDViewComponent|GetIsFirstPerson (Variables|Default|GetViewComp))
      (Class|CCDCharacter|ToggleView))))

(fn OpenItemWheel
  (bind _returnvalue (Game|GetPlayerController 0))
  (if (Utilities|IsValid (Variables|Default|GetItem%20Wheel))
    _
    (else
      (bind _returnvalue_2 (UserInterface|CreateWidget "/Game/_CCD/UI/ItemWheel/WBP_ItemWheel.WBP_ItemWheel_C" (Game|GetPlayerController 0)))
      (Variables|Default|SetItem%20Wheel _returnvalue_2)))
  (CallFunction|SetMousePosMiddle)
  (UserInterface|Viewport|AddtoViewport (Variables|Default|GetItem%20Wheel) 0)
  (Input|SetInputModeGameandUI _returnvalue 0 "LockAlways" true false)
  (Variables|/Script/Engine.PlayerController|SetbShowMouseCursor _returnvalue false))

(fn CloseItemWheel
  (bind _returnvalue (Game|GetPlayerController 0))
  (bind _item_wheel (Variables|Default|GetItem%20Wheel))
  (bind (_choose_equip _change_) (Default|ReturnEquipResult _item_wheel))
  (Widget|RemovefromParent _item_wheel)
  (Input|SetInputModeGameOnly _returnvalue false)
  (Variables|/Script/Engine.PlayerController|SetbShowMouseCursor _returnvalue false)
  (if _change_
    (Class|CCDCharacter|SwitchEquipment _choose_equip)))

(fn SetMousePosMiddle
  (bind _returnvalue (Game|GetPlayerController 0))
  (bind (_sizex _sizey) (HUD|GetViewportSize _returnvalue))
  (Class|PlayerController|SetMouseLocation _returnvalue (/ _sizex 2) (/ _sizey 2)))