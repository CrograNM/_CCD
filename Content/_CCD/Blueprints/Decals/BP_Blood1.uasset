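; BP_Blood1 is a decal Blueprint for a washable mess, which can be blood, excrement or water.
; The construction script reads the type from WashableComp and sets the decal material to match, using a bucket water material for water.
; Blood and excrement pass a random index to SetBlood or SetExcrement, but every index currently resolves to the same single material per type.
; The event graph has no runtime logic.
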(event EventBeginPlay)

(event EventTick
  (params (DeltaSeconds :type Float%20%28single-precision%29)))

(fn ConstructionScript
  (bind _returnvalue (Math|Random|RandomIntegerinRange 0 4))
  (switch Utilities|FlowControl|Switch|SwitchonECCD_WashableType (Class|WashableComponent|GetWashableType (Variables|Default|GetWashableComp))
    (:EWT_Blood
      (CallFunction|SetBlood _returnvalue))
    (:EWT_Excrement
      (CallFunction|SetExcrement _returnvalue))
    (:EWT_Water
      (Rendering|Components|Decal|SetDecalMaterial (Variables|Default|GetDecal) "/Game/_CCD/Meshes/_Decal/MI_BucketWater.MI_BucketWater"))))

(fn SetBlood
  (params (Type_Random :type Integer))
  ;[1 0 0] Blood
  (switch int Type_Random
    (:Default
      (Rendering|Components|Decal|SetDecalMaterial (Variables|Default|GetDecal) "/Game/_CCD/Meshes/_Decal/MI_Blood_01.MI_Blood_01" :!label _label))
    (:0
      (goto _label))
    (:1
      (Rendering|Components|Decal|SetDecalMaterial (Variables|Default|GetDecal) "/Game/_CCD/Meshes/_Decal/MI_Blood_01.MI_Blood_01" :!label _label_2))
    (:2
      (goto _label_2))
    (:3
      (goto _label_2))
    (:4
      (goto _label_2))))

(fn SetExcrement
  (params (Type%20Random :type Integer))
  ;[1 0.9391 0] Excrement
  (switch int Type%20Random
    (:Default
      (Rendering|Components|Decal|SetDecalMaterial (Variables|Default|GetDecal) "/Game/_CCD/Meshes/_Decal/MI_Excrement_01.MI_Excrement_01" :!label _label))
    (:0
      (goto _label))
    (:1
      (Rendering|Components|Decal|SetDecalMaterial (Variables|Default|GetDecal) "/Game/_CCD/Meshes/_Decal/MI_Excrement_01.MI_Excrement_01" :!label _label_2))
    (:2
      (goto _label_2))
    (:3
      (goto _label_2))
    (:4
      (goto _label_2))))