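; Player controller that gives the local player a tablet overlay and an ESC menu.
; On BeginPlay it adds the system input mapping context and creates both widgets, with the tablet starting hidden in the viewport.
; Holding the tablet input shows and refreshes the tablet, and releasing hides it.
; The menu input or 0 key toggles the menu, switching input mode and mouse cursor to match.
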(event Input|EnhancedActionEvents|EnhancedInputActionIA_OpenMenu
  (params (ActionValue :type Vector%202D%20Structure) (ElapsedSeconds :type Float%20%28double-precision%29) (TriggeredSeconds :type Float%20%28double-precision%29) (InputAction :type Input%20Action%20Object%20Reference :default "/Game/_CCD/Input/IA_OpenMenu.IA_OpenMenu"))
  (:Started
    (if (Variables|Default|GetIsMenuOpen)
      (CallFunction|CloseMenu)
      (else
        (CallFunction|OpenMenu)))))

(event Input|EnhancedActionEvents|EnhancedInputActionIA_OpenTablet
  (params (ActionValue :type Boolean) (ElapsedSeconds :type Float%20%28double-precision%29) (TriggeredSeconds :type Float%20%28double-precision%29) (InputAction :type Input%20Action%20Object%20Reference :default "/Game/_CCD/Input/IA_OpenTablet.IA_OpenTablet"))
  (bind _tablet (Variables|Default|GetTablet))
  (:Started
    (Widget|SetVisibility _tablet "Visible")
    (Default|UpdateTablet _tablet))
  (:Completed
    (Widget|SetVisibility _tablet "Hidden")))

(event EventBeginPlay
  (if (Pawn|IsLocalPlayerController)
    (Input|AddMappingContext (PlayerController|LocalPlayerSubsystems|GetEnhancedInputLocalPlayerSubsystem self) "/Game/_CCD/Input/IMC_System.IMC_System" 100 "(bIgnoreAllPressedKeysUntilRelease=True,bForceImmediately=False,bNotifyUserSettings=False)")
    (Utilities|FlowControl|Sequence
      (:then_0
        (bind _returnvalue (UserInterface|CreateWidget "/Game/_CCD/UI/Tablet/WBP_Tablet.WBP_Tablet_C" self))
        (bind _output_get (Variables|Default|SetTablet _returnvalue))
        (UserInterface|Viewport|AddtoViewport _output_get 0)
        (Widget|SetVisibility _output_get "Hidden"))
      (:then_1
        (bind _returnvalue_2 (UserInterface|CreateWidget "/Game/_CCD/UI/ESC/WBP_ESCMenu.WBP_ESCMenu_C" self))
        (Variables|Default|SetMenu _returnvalue_2)))))

(event Input|KeyboardEvents|0
  (params (Key :type Key%20Structure))
  (:Pressed
    (if (Variables|Default|GetIsMenuOpen)
      (CallFunction|CloseMenu)
      (else
        (CallFunction|OpenMenu)))))

(fn ConstructionScript)

(fn OpenMenu
  (if (Utilities|IsValid (Variables|Default|GetMenu))
    _
    (else
      (bind _returnvalue (UserInterface|CreateWidget "/Game/_CCD/UI/ESC/WBP_ESCMenu.WBP_ESCMenu_C" self))
      (Variables|Default|SetMenu _returnvalue)))
  (UserInterface|Viewport|AddtoViewport (Variables|Default|GetMenu) 0)
  (Input|SetInputModeGameandUI self 0 "DoNotLock" true true)
  (Variables|Default|SetbShowMouseCursor true)
  (Variables|Default|SetIsMenuOpen true))

(fn CloseMenu
  (Widget|RemovefromParent (Variables|Default|GetMenu))
  (Input|SetInputModeGameOnly self true)
  (Variables|Default|SetbShowMouseCursor false)
  (Variables|Default|SetIsMenuOpen false))