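; BP_173 is an SCP-173 actor that can test whether the player is observing it; its event graph and construction script are empty.
; CheckIfObserved first uses a dot product to check that the actor lies within a forward cone of the player camera.
; It then line-traces on Visibility from the camera to each listed mesh socket, ignoring itself, and returns true at the first unobstructed one.
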(event EventBeginPlay)

(event Collision|EventActorBeginOverlap
  (params (OtherActor :type Actor%20Object%20Reference)))

(event EventTick
  (params (DeltaSeconds :type Float%20%28single-precision%29)))

(fn ConstructionScript)

(fn CheckifObserved
  (bind _returnvalue (Game|GetPlayerCameraManager 0))
  (if (> (Math|Vector|DotProduct (Math|Vector|GetForwardVector (Camera|GetCameraRotation _returnvalue)) (Math|Vector|Normalize (- (Transformation|GetActorLocation) (Camera|GetCameraLocation _returnvalue)))) 0.7)
    (for _array_element (Variables|Default|GetSocketNames)
      (bind _returnvalue_2 (Collision|LineTraceByChannel (Camera|GetCameraLocation (Game|GetPlayerCameraManager 0)) (Transformation|GetSocketLocation (Variables|Character|GetMesh) _array_element) "TraceTypeQuery1" false (Utilities|Array|MakeArray self) "None"))
      (if (not _returnvalue_2)
        (return true)))
    (return false)
    (else
      (return false))))